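; BP_Player is the player Blueprint that handles object grabbing and the pause menu.
; Pressing and releasing the Grab input action calls Grab and Release on its Grabber.
; Escape drives a FlipFlop that either creates a Pause widget, pauses the game and shows the mouse cursor, or removes the widget, unpauses and hides the cursor.
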(event EventBeginPlay)

(event Collision|EventActorBeginOverlap
  (params (OtherActor :type Actor%20Object%20Reference)))

(event EventTick
  (params (DeltaSeconds :type Float%20%28single-precision%29)))

(event Input|ActionEvents|InputActionGrab
  (params (Key :type Key%20Structure :default "None"))
  (:Pressed
    (Class|Grabber|Grab (Variables|Default|GetGrabber)))
  (:Released
    (Class|Grabber|Release (Variables|Default|GetGrabber))))

(event Input|KeyboardEvents|Escape
  (params (Key :type Key%20Structure :default "None"))
  (bind _returnvalue (Game|GetPlayerController 0))
  (:Pressed
    (Utilities|FlowControl|FlipFlop
      (:A
        (bind _returnvalue_2 (UserInterface|CreateWidget "/Game/Pause_Menu/Pause.Pause_C"))
        (UserInterface|Viewport|AddtoViewport _returnvalue_2 0)
        (Game|SetGamePaused true)
        (Variables|/Script/Engine.PlayerController|SetbShowMouseCursor _returnvalue true))
      (:B
        (Widget|RemovefromParent _returnvalue_2)
        (Game|SetGamePaused false)
        (Variables|/Script/Engine.PlayerController|SetbShowMouseCursor _returnvalue false)))))

(fn ConstructionScript
  (|CallParentFunction))